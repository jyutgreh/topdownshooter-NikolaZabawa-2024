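; Player marine character that moves, turns with the mouse and fires an assault rifle, showing a HUD on begin play.
; The fire input toggles the muzzle flash particle and firing sound, with a closing shot sound on release; no hit logic exists.
; Each tick, mouse velocity above a dead zone becomes a yaw angle toward which control rotation interpolates.
; AnyDamage is empty, and the health-based death check never runs.
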(event `InputAction|PEWPEWPEW!`
  (params (Key :type "Key Structure"))
  ;[0.5953 0.5377 1] shootin
  (:`Pressed`
    ;;[0.1635 0.1028 0.5781] animation
    (`ActorComponent.Activate` (`self.P_AssaultRifle_MF`) false)
    ;;[0.2598 0.3744 1] sound
    (bind _returnvalue (`GameplayStatics.SpawnSound2D` "/Game/Sounds/Weapon_AssaultRifle/Stereo/pewpewpew.pewpewpew" 1.0 1.0 0.0 null))
    (set `self.WeaponSound` _returnvalue))
  (:`Released`
    (`ActorComponent.Deactivate` (`self.P_AssaultRifle_MF`))
    (`AudioComponent.Stop` (`self.WeaponSound`))
    (`GameplayStatics.SpawnSound2D` "/Game/Sounds/Weapon_AssaultRifle/Stereo/pew-.pew-" 1.0 1.0 0.0 null)))

(event `InputAxis|MoveForwardBack`
  (params (AxisValue :type "Float (single-precision)"))
  ;[1 0.7334 0.3291] ruszanie postacią
  (`self.AddMovementInput` (`self.GetActorForwardVector` (`GameplayStatics.GetPlayerController` 0)) AxisValue))

(event `self.ReceiveBeginPlay`
  ;[1 0.4587 0.7001] UI widget
  (bind _returnvalue (`|CreateWidget` "/Game/UI/W_PlayerHUD_01.W_PlayerHUD_01_C" null self))
  (`UserWidget.AddToViewport` _returnvalue 0))

(event `self.ReceiveAnyDamage`
  (params (Damage :type "Float (single-precision)") (DamageType :type "DamageType Object Reference") (InstigatedBy :type "Controller Object Reference") (DamageCauser :type "Actor Object Reference")))

(event `InputAxis|MoveLeftRight`
  (params (AxisValue :type "Float (single-precision)"))
  ;[1 0.7334 0.3291] ruszanie postacią
  (`self.AddMovementInput` (`self.GetActorRightVector` (`GameplayStatics.GetPlayerController` 0)) AxisValue))

(event `self.ReceiveTick`
  (params (DeltaSeconds :type "Float (single-precision)"))
  ;[1 0.7334 0.3291] ruszanie postacią
  ;;[1 0.5 0.2147] obrót postaci
  (`self.Update Character Rotation`))

(fn `IsMouseAboveDeadZone`
  (returns (ReturnValue :type Boolean))
  (return (> (`KismetMathLibrary.VSize2D` (`self.MouseVelocity`)) (`self.DeadZone`))))

(fn `MouseVelocity`
  (returns (ReturnValue :type "Vector2D Structure"))
  (bind (_deltax _deltay) (`PlayerController.GetInputMouseDelta` (`GameplayStatics.GetPlayerController` 0)))
  (return (/ (`KismetMathLibrary.MakeVector2D` _deltax _deltay) (`GameplayStatics.GetWorldDeltaSeconds`))))

(fn `Update Character Rotation`
  (bind (_returnvalue_x _returnvalue_y) (`KismetMathLibrary.BreakVector2D` (`self.MouseVelocity`)))
  (bind _returnvalue (`GameplayStatics.GetPlayerController` 0))
  (if (`self.IsMouseAboveDeadZone`)
    (`Controller.SetControlRotation` _returnvalue (`KismetMathLibrary.RInterpTo` (`Controller.GetControlRotation` _returnvalue) (`KismetMathLibrary.MakeRotator` 0.0 0.0 (`KismetMathLibrary.DegAtan2` _returnvalue_x _returnvalue_y)) (`GameplayStatics.GetWorldDeltaSeconds`) (`self.Interp Speed`)))))

(fn `UserConstructionScript`)