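; BP_Spider is an enemy spider that chases the player and attacks up close.
; A repeating AIMoveTo drives pursuit, while Tick checks distance and pauses movement during the attack montage.
; Damage reduces clamped health and passes a zero-health Death flag to KillSpider.
; Any hit, even non-lethal, disables movement and collision and destroys the actor after a delay, since nothing branches on that flag.
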(event `self.ReceiveBeginPlay`
  ;[1 1 1] following the player
  (`|AIMoveTo` self (0.0 0.0 0.0) (`GameplayStatics.GetPlayerCharacter` 0) :!label _label
    (:`OnSuccess`
      (`KismetSystemLibrary.Delay` 0.2)
      (goto _label))))

(event `self.ReceiveTick`
  (params (DeltaSeconds :type "Float (single-precision)"))
  ;[1 1 1] attack
  (if (and (`self.isAttackRange`) (not (`self.IsAttacking`)))
    (`ActorComponent.Deactivate` (`self.CharacterMovement`))
    (`|PlayMontage` (`self.Mesh`) "/Game/Characters/Enemy_Great_Spider/Animations/AM_SpiderAttack.AM_SpiderAttack" 0.5
      (:`OnCompleted`
        (`ActorComponent.Activate` (`self.CharacterMovement`) false)))))

(event `self.ReceiveAnyDamage`
  (params (Damage :type "Float (single-precision)") (DamageType :type "DamageType Object Reference") (InstigatedBy :type "Controller Object Reference") (DamageCauser :type "Actor Object Reference"))
  ;[1 1 1] health & death
  (bind _output_get (set `self.Health` (`KismetMathLibrary.FClamp` (- (`self.Health`) Damage) 0.0 100.0)))
  (`self.Kill Spider` (== _output_get 0.0))
  (`KismetSystemLibrary.Delay` 5.0)
  (`self.K2_DestroyActor`))

(fn `IsAttacking`
  (returns (ReturnValue :type Boolean))
  (return (`AnimInstance.Montage_IsPlaying` (`SkeletalMeshComponent.GetAnimInstance` (`self.Mesh`)) "/Game/Characters/Enemy_Great_Spider/Animations/AM_SpiderAttack.AM_SpiderAttack")))

(fn `isAttackRange`
  (returns (ReturnValue :type Boolean))
  (return (< (`self.GetDistanceTo` (`GameplayStatics.GetPlayerCharacter` 0)) (`self.AttackRange`))))

(fn `Kill Spider`
  (params (Death :type Boolean))
  (set `self.Death` Death)
  (`ActorComponent.Deactivate` (`self.CharacterMovement`))
  (`self.SetActorEnableCollision` false))

(fn `UserConstructionScript`)